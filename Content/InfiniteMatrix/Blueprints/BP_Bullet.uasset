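; BP_Bullet is a projectile actor that moves via ProjectileMovement and destroys itself when it hits or overlaps a BP_Tunnel.
; On BeginPlay it uses its Player1ref, falling back to casting player pawn 0 to BP_Player, and sets its initial and max speed to a multiple of the player's ForwardSpeed.
; It also gives its sphere mesh a random material from a fixed set of six.
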(event `self.Sphere.OnComponentHit`
  (params (HitComponent :type "PrimitiveComponent Object Reference") (OtherActor :type "Actor Object Reference") (OtherComp :type "PrimitiveComponent Object Reference") (NormalImpulse :type "Vector Structure") (Hit :type "HitResult Structure (by ref)"))
  (if (== (`GameplayStatics.GetObjectClass` OtherActor) "/Game/InfiniteMatrix/Blueprints/BP_Tunnel.BP_Tunnel_C")
    (`self.K2_DestroyActor`)))

(event `self.SphereCol.OnComponentBeginOverlap`
  (params (OverlappedComponent :type "PrimitiveComponent Object Reference") (OtherActor :type "Actor Object Reference") (OtherComp :type "PrimitiveComponent Object Reference") (OtherBodyIndex :type Integer) (bFromSweep :type Boolean) (SweepResult :type "HitResult Structure (by ref)"))
  (if (== (`GameplayStatics.GetObjectClass` OtherActor) "/Game/InfiniteMatrix/Blueprints/BP_Tunnel.BP_Tunnel_C")
    (`self.K2_DestroyActor`)))

(event `self.ReceiveBeginPlay`
  (`/Engine/EditorBlueprintResources/StandardMacros.IsValid` (`self.player1ref`)
    (:`Is Valid`
      _)
    (:`Is Not Valid`
      (bind _asbp_player (cast `/Game/InfiniteMatrix/Blueprints/BP_Player` (`GameplayStatics.GetPlayerPawn` 0)))
      (bind _output_get (set `self.player1ref` _asbp_player))))
  (bind _output_get_2 (set `ProjectileMovementComponent.InitialSpeed` (* (`/Game/InfiniteMatrix/Blueprints/BP_Player.ForwardSpeed` _output_get) 5.0) (`self.ProjectileMovement`)))
  (set `ProjectileMovementComponent.MaxSpeed` _output_get_2 (`self.ProjectileMovement`))
  (`PrimitiveComponent.SetMaterial` (`self.Sphere`) 0 (select `int` (`KismetMathLibrary.RandomIntegerInRange` 0 5) :`0` "/Engine/VREditor/BasicMeshes/MI_Cube_03.MI_Cube_03" :`1` "/Engine/EditorMaterials/MatineeGroups/MAT_Groups_Right_On_Mat.MAT_Groups_Right_On_Mat" :`2` "/Engine/MapTemplates/Materials/BasicAsset01.BasicAsset01" :`3` "/Engine/MapTemplates/Materials/BasicAsset03.BasicAsset03" :`4` "/Engine/EditorMaterials/WidgetGridVertexColorMaterial_Ma.WidgetGridVertexColorMaterial_Ma" :`5` "/Engine/EditorMaterials/MatineeGroups/MAT_ColorTrack_Mat.MAT_ColorTrack_Mat" :!type "MaterialInterface Object Reference")))

(fn `UserConstructionScript`)